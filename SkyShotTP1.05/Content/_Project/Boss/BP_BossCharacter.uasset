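; Boss character that plays a fight animation and spawns BP_Objective actors from its hands.
; BeginPlay stops the mesh animation; evFight plays Boss_Fight once, waits briefly, then spawns at the left and right hand sockets.
; Both spawns feed a shared counter that re-enters the sequence without delay until its limit, producing a burst, then prints the count.
; The evAttack event is an empty stub.
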(event Custom|evFight
  (bind _mesh (Variables|Character|GetMesh))
  (Components|Animation|PlayAnimation (Variables|Character|GetMesh) "/Game/_Project/Boss/Boss_Fight.Boss_Fight" false)
  (Utilities|FlowControl|Delay 4.0)
  (Utilities|FlowControl|Sequence :!label _label
    (:then_0
      (Game|SpawnActorfromClass "/Game/ThirdPerson/Blueprints/BP_Objective.BP_Objective_C" (Math|Transform|MakeTransform (Transformation|GetSocketLocation _mesh "HandSocket_L") "0, 0, 0" "1.000000,1.000000,1.000000") "Undefined" "MultiplyWithRoot" 0 0))
    (:then_1
      (Game|SpawnActorfromClass "/Game/ThirdPerson/Blueprints/BP_Objective.BP_Objective_C" (Math|Transform|MakeTransform (Transformation|GetSocketLocation _mesh "HandSocket_R") "0, 0, 0" "1.000000,1.000000,1.000000") "Undefined" "MultiplyWithRoot" 0 0)))
  (Math|Integer|IncrementInt (Variables|Default|GetCounter)
    (:%20%20
      (if (<= (Variables|Default|GetCounter) 10)
        (goto _label)
        (else
          (Development|PrintString (Utilities|String|ToString(Integer) (Variables|Default|GetCounter))))))))

(event Custom|evAttack)

(event EventBeginPlay
  (Audio|Components|Audio|Stop (Variables|Character|GetMesh)))

(event Collision|EventActorBeginOverlap
  (params (OtherActor :type Actor%20Object%20Reference)))

(event EventTick
  (params (DeltaSeconds :type Float%20%28single-precision%29)))

(fn ConstructionScript)